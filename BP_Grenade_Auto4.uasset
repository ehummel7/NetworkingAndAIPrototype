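; Grenade actor that is thrown with a given velocity and explodes after a short fixed fuse.
; Throw activates the projectile movement, waits, then spawns the explosion effect, hides the sphere and sets a short lifespan for cleanup.
; A zero-length sphere trace finds nearby Pawns, collects them without duplicates, and sends each a GrenadeHitMessage with the blast location and fixed damage.
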(event `self.ReceiveBeginPlay`)

(event `Throw`
  (params (Velocity :type "Vector Structure"))
  (bind _projectilemovement (`self.ProjectileMovement`))
  (bind _returnvalue (`SceneComponent.K2_GetComponentLocation` (`self.Sphere`)))
  (set `MovementComponent.Velocity` Velocity _projectilemovement)
  (`ActorComponent.Activate` _projectilemovement false)
  (`KismetSystemLibrary.Delay` 0.5)
  (`GameplayStatics.SpawnEmitterAtLocation` "/Game/StarterContent/Particles/P_Explosion.P_Explosion" (`SceneComponent.K2_GetComponentLocation` (`self.Sphere`)))
  (`SceneComponent.SetHiddenInGame` (`self.Sphere`) true false)
  (`self.SetLifeSpan` 3.0)
  (bind (_outhits _returnvalue_2) (`KismetSystemLibrary.SphereTraceMultiForObjects` _returnvalue _returnvalue 50.0 (`|MakeArray` "ObjectTypeQuery3" :!type "EObjectTypeQuery Enum")))
  (if _returnvalue_2
    (for _array_element _outhits
      (`KismetArrayLibrary.Array_AddUnique` (`self.HitActors`) (`.HitActor` (`GameplayStatics.BreakHitResult` _array_element))))
    (for _array_element_2 (`self.HitActors`)
      (message `/Game/FirstPersonBP/Blueprints/BPI_Character.GrenadeHit` _array_element_2 _returnvalue 100.0))))

(fn `UserConstructionScript`)